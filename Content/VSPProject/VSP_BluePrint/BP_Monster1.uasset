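; BP_Monster1 is a monster actor that homes in on the player.
; On BeginPlay it casts player character 0 to BP_Player and stores it as the target.
; Each Tick it turns toward the target using only the look-at yaw and roll, then steps along the full 3D look-at direction.
; Movement is a fixed offset per frame, without sweep, delta-time scaling or navigation.
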(event EventTick
  (params (DeltaSeconds :type Float%20%28single-precision%29))
  (bind _returnvalue (Transformation|GetActorLocation))
  (bind _target (Variables|Default|GetTarget))
  (bind _returnvalue_2 (Transformation|GetActorLocation _target))
  (bind _returnvalue_3 (Math|Rotator|FindLookatRotation _returnvalue _returnvalue_2))
  (Utilities|IsValid _target
    (:Is%20Valid
      (Transformation|SetActorRotation (Math|Rotator|MakeRotator (.roll _returnvalue_3) 0.0 (.yaw _returnvalue_3)))
      (Transformation|AddActorWorldOffset (* (Math|Vector|GetForwardVector (Math|Rotator|FindLookatRotation (Transformation|GetActorLocation) (Transformation|GetActorLocation (Variables|Default|GetTarget)))) 2.0)))))

(event EventBeginPlay
  (bind _asbp_player (Utilities|Casting|CastToBP_Player (Game|GetPlayerCharacter 0)))
  (Variables|Default|SetTarget _asbp_player))

(fn ConstructionScript)